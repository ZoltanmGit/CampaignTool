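; BP_Character is a character Blueprint that shows its health on a selected-portrait HUD widget.
; On BeginPlay, if its controller is a PlayerController, it creates WBP_SelectedPortrait for that player, stores it as PortraitUI and adds it to the viewport.
; The OnHealthChange event reads current health and percentage from CharacterHealth and pushes them to the portrait's text and progress bar.
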(event EventBeginPlay
  (bind _asplayer_controller (Utilities|Casting|CastToPlayerController (Pawn|GetController self)))
  (bind _returnvalue (UserInterface|CreateWidget "/Game/UI/WBP_SelectedPortrait.WBP_SelectedPortrait_C" _asplayer_controller))
  (bind _output_get (Variables|Default|SetPortraitUI _returnvalue))
  (UserInterface|Viewport|AddtoViewport _output_get 0))

(event EventOnHealthChange
  ;[1 1 1] Health Change
  (bind _returnvalue (Class|HealthComponent|GetCurrentHealth (Variables|Default|GetCharacterHealth)))
  (Rendering|Components|TextRender|SetText (Variables|/Game/UI/WBP_SelectedPortrait.WBP_SelectedPortrait_C|GethealthText (Variables|Default|GetPortraitUI)) (Utilities|Text|ToText(Float) _returnvalue "HalfToEven"))
  (bind _returnvalue_2 (Class|HealthComponent|GetHealthPercent (Variables|Default|GetCharacterHealth)))
  (Progress|SetPercent (Variables|/Game/UI/WBP_SelectedPortrait.WBP_SelectedPortrait_C|GethealthProgressBar (Variables|Default|GetPortraitUI)) _returnvalue_2))

(fn ConstructionScript)