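; General ability that resolves a main-hand melee attack with tabletop-style dice rules.
; On execute, a d20 roll plus the owner's attack bonus is compared to the target's armor class.
; On a hit, the equipped weapon supplies damage type and dice, using versatile dice when the offhand is empty, and damage plus bonus goes to the target's health component.
; A natural 20 only sets a critical flag, unused in this graph.
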(event EventOnExecute
  (bind _ownercharacter (Variables|Default|GetOwnerCharacter))
  ;[1 1 1] Determinte hit
  (bind _returnvalue (Class|DiceRoller|Roll (Variables|/Script/CampaignTool.BaseCharacter|GetDiceRoller (Variables|Default|GetOwnerCharacter)) 20 1 false false))
  (if (== _returnvalue 20)
    (Variables|Default|SetIsCriticalHit true))
  (bind _returnvalue_2 (Class|CharacterInventoryComponent|GetMainAttackBonus (Variables|/Script/CampaignTool.BaseCharacter|GetCharacterInventory (Variables|Default|GetOwnerCharacter))))
  (bind _returnvalue_3 (Class|CharacterInventoryComponent|GetArmorClass (Variables|/Script/CampaignTool.BaseCharacter|GetCharacterInventory (Variables|Default|GetTargetCharacter))))
  (Development|PrintString 0 (Utilities|String|Append "Attack: Roll " (Utilities|String|ToString(Integer) _returnvalue) " + " (Utilities|String|ToString(Integer) _returnvalue_2) " against " (Utilities|String|ToString(Integer) _returnvalue_3)) true true "(R=0.101539,G=1.000000,B=0.000000,A=1.000000)" 1e+01)
  (if (<= _returnvalue_3 (+ _returnvalue_2 _returnvalue))
    (Development|PrintString 0 "Attack hit")
    ;[1 1 1] If a hit occurs, get weapon
    (bind _returnvalue_4 (Class|CharacterInventoryComponent|GetEquipment (Variables|/Script/CampaignTool.BaseCharacter|GetCharacterInventory (Variables|Default|GetOwnerCharacter)) "EquipmentSlot_MainHand"))
    (bind _asbase_weapon_item (Utilities|Casting|CastToBaseWeaponItem _returnvalue_4)
      (:then
        (Variables|Default|SetUsedDamageType (Variables|/Script/CampaignTool.BaseWeaponItem|GetDamageType _asbase_weapon_item))
        (if (Variables|/Script/CampaignTool.BaseWeaponItem|GetbIsVersatile _asbase_weapon_item)
          ;[1 1 1] If Versatile we check if it's applicable
          (if (Variables|/Script/CampaignTool.CharacterInventoryComponent|GetbHasOffhand (Variables|/Script/CampaignTool.BaseCharacter|GetCharacterInventory (Variables|Default|GetOwnerCharacter)))
            ;[1 1 1] If not we just assign values
            (Variables|Default|SetUsedDamageDie (Variables|/Script/CampaignTool.BaseWeaponItem|GetDamageDie _asbase_weapon_item) :!label _label)
            (Variables|Default|SetUsedDamageMultiplier (Variables|/Script/CampaignTool.BaseWeaponItem|GetDamageDieMultiplier _asbase_weapon_item))
            (else
              (Variables|Default|SetUsedDamageDie (Variables|/Script/CampaignTool.BaseWeaponItem|GetVersatileDamageDie _asbase_weapon_item))
              (Variables|Default|SetUsedDamageMultiplier (Variables|/Script/CampaignTool.BaseWeaponItem|GetVersatileDieMultiplier _asbase_weapon_item))))
          (else
            (goto _label)))
        ;[1 1 1] Determine Damage
        (bind _returnvalue_5 (Class|DiceRoller|Roll (Variables|/Script/CampaignTool.BaseCharacter|GetDiceRoller _ownercharacter) (Variables|Default|GetUsedDamageDie) (Variables|Default|GetUsedDamageMultiplier) false false))
        (bind _returnvalue_6 (Class|CharacterInventoryComponent|GetMainDamageBonus (Variables|/Script/CampaignTool.BaseCharacter|GetCharacterInventory _ownercharacter)))
        (Variables|Default|SetUsedDamage (+ _returnvalue_5 _returnvalue_6))
        ;[1 1 1] Apply Damage
        (Class|HealthComponent|HandleDamage (Variables|/Script/CampaignTool.BaseCharacter|GetCharacterHealth (Variables|Default|GetTargetCharacter)) (Variables|Default|GetOwnerCharacter) (Math|Conversions|ToFloat(Integer) (Variables|Default|GetUsedDamage)) (Variables|Default|GetUsedDamageType))
        (Development|PrintString 0 (Utilities|String|Append "Dealt " (Utilities|String|ToString(Float) (Math|Conversions|ToFloat(Integer) (Variables|Default|GetUsedDamage))) " Damage.") true true "(R=1.000000,G=0.000000,B=0.019686,A=1.000000)" 1e+01))
      (:CastFailed
        (Development|PrintString 0 "Mainhand cast failed")))
    (else
      (Development|PrintString 0 "Attack did not hit."))))