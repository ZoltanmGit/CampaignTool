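; Dragonborn lightning breath ability that deals lightning damage to the characters it affects, following tabletop-style dice and saving throw rules.
; On execute, it rolls d6 damage once, and each affected character makes a Constitution save against a DC built from the owner's Constitution modifier and proficiency bonus.
; A successful save halves the damage, and the internal usage number is set to zero afterwards.
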(event EventOnExecute
  (bind _ownercharacter (Variables|Default|GetOwnerCharacter))
  (bind _characterattributes (Variables|/Script/CampaignTool.BaseCharacter|GetCharacterAttributes _ownercharacter))
  (bind _returnvalue (Class|DiceRoller|Roll (Variables|/Script/CampaignTool.BaseCharacter|GetDiceRoller (Variables|Default|GetOwnerCharacter)) 6 2 false false))
  (bind _returnvalue_2 (Class|AttributesComponent|GetModifier _characterattributes "Constitution"))
  (bind _returnvalue_3 (Class|AttributesComponent|GetProficiencyBonus _characterattributes))
  (for _array_element (Variables|Default|GetAffectedCharacters)
    (if (Class|BaseCharacter|MakeSave _array_element "Constitution" (+ 8 _returnvalue_2 _returnvalue_3))
      (Class|HealthComponent|HandleDamage (Variables|/Script/CampaignTool.BaseCharacter|GetCharacterHealth _array_element) 0 (/ (Math|Conversions|ToFloat(Integer) _returnvalue) 2.0) "Lightning")
      (else
        (Class|HealthComponent|HandleDamage (Variables|/Script/CampaignTool.BaseCharacter|GetCharacterHealth _array_element) 0 (Math|Conversions|ToFloat(Integer) _returnvalue) "Lightning"))))
  (Variables|Default|SetInternalUsageNumber 0))