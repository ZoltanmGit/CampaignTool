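; Fighter Second Wind ability that heals the owning character when executed.
; On execute it rolls a ten-sided die through the owner's DiceRoller and adds the character's Fighter class level.
; The total goes to CharacterHealth's HandleDamage as Healing damage with the owner as instigator, then a debug message prints.
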(event EventOnExecute
  (bind _ownercharacter (Variables|Default|GetOwnerCharacter))
  (bind _returnvalue (Class|DiceRoller|Roll (Variables|/Script/CampaignTool.BaseCharacter|GetDiceRoller (Variables|Default|GetOwnerCharacter)) 10 1 false false))
  (bind _returnvalue_2 (Class|AttributesComponent|GetClassLevel (Variables|/Script/CampaignTool.BaseCharacter|GetCharacterAttributes (Variables|Default|GetOwnerCharacter)) "Fighter"))
  (Class|HealthComponent|HandleDamage (Variables|/Script/CampaignTool.BaseCharacter|GetCharacterHealth _ownercharacter) _ownercharacter (Math|Conversions|ToFloat(Integer) (+ _returnvalue_2 _returnvalue)) "Healing")
  (Development|PrintString 0 "Second Wind Healed"))