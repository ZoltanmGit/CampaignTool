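; Main-hand melee attack ability that resolves a d20 attack roll from the owner against the target's armor class.
; On a hit it rolls the equipped weapon's damage die, doubling the dice on a natural 20 and adding any magic bonus.
; The damage-dealing call to the target's health component is disconnected, so the computed damage is never applied; misses only print a message.
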(event EventOnExecute
  (bind _ownercharacter (Variables|Default|GetOwnerCharacter))
  (bind _diceroller (Variables|/Script/CampaignTool.BaseCharacter|GetDiceRoller _ownercharacter))
  ;[1 1 1] Determinte hit
  (bind _returnvalue (Class|DiceRoller|Roll _diceroller 20 1 false false))
  (bind _returnvalue_2 (Class|CharacterInventoryComponent|GetMainAttackBonus (Variables|/Script/CampaignTool.BaseCharacter|GetCharacterInventory _ownercharacter)))
  (bind _returnvalue_3 (Class|CharacterInventoryComponent|GetArmorClass (Variables|/Script/CampaignTool.BaseCharacter|GetCharacterInventory (Variables|Default|GetTargetCharacter))))
  (if (<= _returnvalue_3 (+ _returnvalue_2 _returnvalue))
    ;[1 1 1] Init weapon locally
    (bind _returnvalue_4 (Class|CharacterInventoryComponent|GetMainHandWeapon (Variables|/Script/CampaignTool.BaseCharacter|GetCharacterInventory (Variables|Default|GetOwnerCharacter))))
    (Utilities|IsValid _returnvalue_4
      (:Is%20Valid
        (bind _output_get (Variables|Default|SetWeapon _returnvalue_4))
        (Variables|Default|SetMultiplier (Variables|/Script/CampaignTool.BaseWeaponItem|GetDamageDieMultiplier _output_get))
        ;[1 1 1] Check if Critical Hit
        (if (== _returnvalue 20)
          ;[1 1 1] If it's crit, we double the damage die
          (Variables|Default|SetIsCriticalHit true)
          (Variables|Default|SetMultiplier (* (Variables|Default|GetMultiplier) 2)))
        ;[1 1 1] Determine Damage
        (bind _returnvalue_5 (Class|DiceRoller|Roll _diceroller (Variables|/Script/CampaignTool.BaseWeaponItem|GetDamageDie (Variables|Default|GetWeapon)) (Variables|Default|GetMultiplier) false false))
        (Variables|Default|SetDamage _returnvalue_5)
        ;[0.3016 0.2639 1] Add magic modifier
        (if (Variables|/Script/CampaignTool.BaseWeaponItem|GetbIsMagical (Variables|Default|GetWeapon))
          (Variables|Default|SetDamage (+ (Variables|Default|GetDamage) (Variables|/Script/CampaignTool.BaseWeaponItem|GetMagicBonus (Variables|Default|GetWeapon))))))
      (:Is%20Not%20Valid
        (Development|PrintString 0 "Weapon is NONE")))
    (else
      (Development|PrintString 0 "Attack did not hit."))))