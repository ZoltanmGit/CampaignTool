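; Cure Wounds ability Blueprint that applies a dice-rolled amount to the target character's health when executed.
; It rolls a single d8 through the owner character's DiceRoller and passes the result to the target's CharacterHealth via HandleDamage.
; The effect goes through the damage path with the ability's DamageType rather than a separate heal call, then prints the rolled amount for debugging.
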(event EventOnExecute
  (bind _returnvalue (Class|DiceRoller|Roll (Variables|/Script/CampaignTool.BaseCharacter|GetDiceRoller (Variables|Default|GetOwnerCharacter)) 8 1))
  (Class|HealthComponent|HandleDamage (Variables|/Script/CampaignTool.BaseCharacter|GetCharacterHealth (Variables|Default|GetTargetCharacter)) (Math|Conversions|ToFloat(Integer) _returnvalue) (Variables|Default|GetDamageType))
  (Development|PrintString 0 (Utilities|String|Append "Cure Wounds: " (Utilities|String|ToString(Float) (Math|Conversions|ToFloat(Integer) _returnvalue)))))