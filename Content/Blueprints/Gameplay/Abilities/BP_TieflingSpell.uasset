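; BP_TieflingSpell is an ability that makes a dice-based spell attack from its owner character on a target character.
; On execute it zeroes InternalUsageNumber and rolls a d20 through the owner's DiceRoller against the target inventory's armor class.
; When armor class is greater than or equal to the roll, a d8 roll is dealt as typed damage through the target's CharacterHealth.
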(event EventOnExecute
  (Variables|Default|SetInternalUsageNumber 0)
  (bind _returnvalue (Class|DiceRoller|Roll (Variables|/Script/CampaignTool.BaseCharacter|GetDiceRoller (Variables|Default|GetOwnerCharacter)) 20 1 false false))
  (bind _returnvalue_2 (Class|CharacterInventoryComponent|GetArmorClass (Variables|/Script/CampaignTool.BaseCharacter|GetCharacterInventory (Variables|Default|GetTargetCharacter))))
  (if (>= _returnvalue_2 _returnvalue)
    (bind _returnvalue_3 (Class|DiceRoller|Roll (Variables|/Script/CampaignTool.BaseCharacter|GetDiceRoller (Variables|Default|GetOwnerCharacter)) 8 1 false false))
    (Class|HealthComponent|HandleDamage (Variables|/Script/CampaignTool.BaseCharacter|GetCharacterHealth (Variables|Default|GetTargetCharacter)) 0 (Math|Conversions|ToFloat(Integer) _returnvalue_3) (Variables|Default|GetDamageType))))