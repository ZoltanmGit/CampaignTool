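; Base character Blueprint that shows its health on a selected-portrait HUD widget.
; On BeginPlay it casts its controller to PlayerController, then creates WBP_SelectedPortrait and adds it to the viewport.
; OnHealthChange reads the CharacterHealth component and pushes the health ratio to the portrait's progress bar and current health to its text.
; Failed casts and invalid references only print error strings.
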(event EventBeginPlay
  (bind _asplayer_controller (Utilities|Casting|CastToPlayerController (Pawn|GetController self))
    (:then
      (bind _returnvalue (UserInterface|CreateWidget "/Game/UI/WBP_SelectedPortrait.WBP_SelectedPortrait_C" _asplayer_controller))
      (bind _output_get (Variables|Default|SetPortait _returnvalue))
      (UserInterface|Viewport|AddtoViewport _output_get 0))
    (:CastFailed
      (Development|PrintString "Controller Cast Failed"))))

(event EventOnHealthChange
  (bind _characterhealth (Variables|Default|GetCharacterHealth))
  (Utilities|IsValid (Variables|Default|GetPortait)
    (:Is%20Valid
      (Utilities|IsValid (Variables|Default|GetCharacterHealth)
        (:Is%20Valid
          (bind _returnvalue (Class|HealthComponent|GetFullHealth _characterhealth))
          (bind _returnvalue_2 (Class|HealthComponent|GetCurrentHealth _characterhealth))
          (Progress|SetPercent (Variables|/Game/UI/WBP_SelectedPortrait.WBP_SelectedPortrait_C|GethealthProgressBar (Variables|Default|GetPortait)) (/ _returnvalue_2 _returnvalue))
          (bind _returnvalue_3 (Class|HealthComponent|GetCurrentHealth (Variables|Default|GetCharacterHealth)))
          (Rendering|Components|TextRender|SetText (Variables|/Game/UI/WBP_SelectedPortrait.WBP_SelectedPortrait_C|GethealthText (Variables|Default|GetPortait)) (Utilities|Text|ToText(Float) _returnvalue_3 "HalfToEven")))
        (:Is%20Not%20Valid
          (Development|PrintString "Error: Health Component is invalid"))))
    (:Is%20Not%20Valid
      (Development|PrintString "Error: Portrait Widget is invalid"))))

(fn ConstructionScript)