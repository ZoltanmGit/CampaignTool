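; Player character Blueprint that owns the HUD and aim and movement indicators for a tabletop-style RPG character.
; It creates the UI widget on BeginPlay, attaches it to the possessing player controller, and removes it on unpossession.
; Change events refresh health, stats and inventory from the character's components.
; Pathfinding and ability-aim events spawn or clean up indicators; spellbook construction is an empty stub.
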(event EventBeginPlay
  ;[1 1 1] User Interface
  (bind _returnvalue (UserInterface|CreateWidget "/Game/UI/GameUI/WBP_UserInterface.WBP_UserInterface_C" 0 self))
  (bind _output_get (Variables|Default|SetUI _returnvalue))
  (Widget|SetVisibility _output_get "Collapsed"))

(event EventOnPathfinding
  (params (transform :type Transform))
  (Class|IndicatorActor|SpawnIndicator (Variables|Default|GetIndicator) (.Location (Math|Transform|BreakTransform transform)) "MovementIndicator"))

(event EventOnInventoryOpen
  (bind _ui (Variables|Default|GetUI))
  (bind _wbp_inventory (Variables|/Game/UI/GameUI/WBP_UserInterface.WBP_UserInterface_C|GetWBP_Inventory _ui))
  (Utilities|IsValid _wbp_inventory
    (:Is%20Valid
      (Widget|SetVisibility _wbp_inventory "Visible"))))

(event EventOnInventoryClose
  (bind _ui (Variables|Default|GetUI))
  (bind _wbp_inventory (Variables|/Game/UI/GameUI/WBP_UserInterface.WBP_UserInterface_C|GetWBP_Inventory _ui))
  (Utilities|IsValid _wbp_inventory
    (:Is%20Valid
      (Widget|SetVisibility _wbp_inventory "Collapsed"))))

(event EventOnConstructSpellBook
  (CallFunction|ConstructSpells))

(event EventPossessed
  (params (NewController :type Controller%20Object%20Reference))
  (CallFunction|HandlePossession NewController))

(event EventUnpossessed
  (params (OldController :type Controller%20Object%20Reference))
  (CallFunction|HandleUnpossession OldController))

(event EventCleanupPathfinding
  ;[1 1 1] Effect Indicatiors
  (Class|IndicatorActor|CleanupIndicators (Variables|Default|GetIndicator) "MovementIndicator"))

(event EventOnHealthChange
  ;[1 1 1] User Interface
  (CallFunction|UpdateHealth))

(event EventOnAbilityAim
  (params (transform :type Transform))
  ;[1 1 1] Effect Indicatiors
  (Class|IndicatorActor|SpawnIndicator (Variables|Default|GetIndicator) (.Location (Math|Transform|BreakTransform transform)) "AbilityIndicator"))

(event EventCleanupAbilityIndicators
  ;[1 1 1] Effect Indicatiors
  (Class|IndicatorActor|CleanupIndicators (Variables|Default|GetIndicator) "AbilityIndicator"))

(event EventOnStatChange
  ;[1 1 1] User Interface
  (CallFunction|UpdateStats))

(event EventOnInventoryChange
  (bind _ui (Variables|Default|GetUI))
  (bind _wbp_inventory (Variables|/Game/UI/GameUI/WBP_UserInterface.WBP_UserInterface_C|GetWBP_Inventory _ui))
  ;[1 1 1] User Interface
  (Utilities|IsValid _wbp_inventory
    (:Is%20Valid
      (Default|RefreshInventory _wbp_inventory))))

(fn ConstructionScript)

(fn UpdateStats
  (bind _ui (Variables|Default|GetUI))
  (bind _ui_2 (Variables|Default|GetUI))
  (bind _wbp_statindicator (Variables|/Game/UI/GameUI/WBP_UserInterface.WBP_UserInterface_C|GetWBP_StatIndicator _ui))
  (bind _wbp_statindicator_2 (Variables|/Game/UI/GameUI/WBP_UserInterface.WBP_UserInterface_C|GetWBP_StatIndicator _ui_2))
  (bind _tohittext (Variables|/Game/UI/GameUI/WBP_StatIndicator.WBP_StatIndicator_C|GettoHitText _wbp_statindicator_2))
  (bind _hittext (Variables|/Game/UI/GameUI/WBP_StatIndicator.WBP_StatIndicator_C|GethitText _wbp_statindicator))
  (if (and (Utilities|IsValid (Variables|Default|GetUI)) (Utilities|IsValid (Variables|Default|GetCharacterInventory)))
    ;[1 1 1] Set Armor Class Text
    (bind _returnvalue (Class|CharacterInventoryComponent|GetArmorClass (Variables|Default|GetCharacterInventory)))
    (Rendering|Components|TextRender|SetText (Variables|/Game/UI/GameUI/WBP_StatIndicator.WBP_StatIndicator_C|GetarmorClassText (Variables|/Game/UI/GameUI/WBP_UserInterface.WBP_UserInterface_C|GetWBP_StatIndicator (Variables|Default|GetUI))) (Utilities|Text|ToText(Integer) _returnvalue))
    ;[1 1 1] Set Main Attack Text
    (bind _returnvalue_2 (Class|CharacterInventoryComponent|GetMainAttackBonus (Variables|Default|GetCharacterInventory)))
    (if (>= _returnvalue_2 0)
      (Rendering|Components|TextRender|SetText _tohittext (Utilities|Text|ToText(String) (Utilities|String|Append "+" (Utilities|String|ToString(Integer) _returnvalue_2))))
      (else
        (Rendering|Components|TextRender|SetText _tohittext (Utilities|Text|ToText(Integer) _returnvalue_2))))
    ;[1 1 1] Set Main Attack Text
    (bind _returnvalue_3 (Class|CharacterInventoryComponent|GetMainDamageBonus (Variables|Default|GetCharacterInventory)))
    (if (>= _returnvalue_3 0)
      (Rendering|Components|TextRender|SetText _hittext (Utilities|Text|ToText(String) (Utilities|String|Append "+" (Utilities|String|ToString(Integer) _returnvalue_3))))
      (else
        (Rendering|Components|TextRender|SetText _hittext (Utilities|Text|ToText(Integer) _returnvalue_3))))
    ;[1 1 1] Update speed text in portrait widget
    (Rendering|Components|TextRender|SetText (Variables|/Game/UI/GameUI/WBP_StatIndicator.WBP_StatIndicator_C|GetspeedText (Variables|/Game/UI/GameUI/WBP_UserInterface.WBP_UserInterface_C|GetWBP_StatIndicator (Variables|Default|GetUI))) (Utilities|Text|ToText(String) (Utilities|String|Append (Utilities|String|ToString(Integer) (Math|Float|Round (* 5 (Variables|Default|GetCurrentSpeed)))) "ft.")))
    ;[1 1 1] Set Spell Num Text
    (Rendering|Components|TextRender|SetText (Variables|/Game/UI/GameUI/WBP_StatIndicator.WBP_StatIndicator_C|GetspellSlotText (Variables|/Game/UI/GameUI/WBP_UserInterface.WBP_UserInterface_C|GetWBP_StatIndicator (Variables|Default|GetUI))) (Utilities|Text|ToText(Integer) (Variables|Default|GetSpellSlotNum)))
    (else
      ;[1 1 1] Debug Logging
      (Development|PrintString "BP_PlayerCharacter - Update Stats(): UI or CharacterInventory is not valid"))))

(fn UpdateHealth
  (if (and (Utilities|IsValid (Variables|Default|GetUI)) (Utilities|IsValid (Variables|Default|GetCharacterHealth)))
    ;[1 1 1] Set Health Text
    (bind _returnvalue (Class|HealthComponent|GetCurrentHealth (Variables|Default|GetCharacterHealth)))
    (Rendering|Components|TextRender|SetText (Variables|/Game/UI/GameUI/WBP_StatIndicator.WBP_StatIndicator_C|GethealthText (Variables|/Game/UI/GameUI/WBP_UserInterface.WBP_UserInterface_C|GetWBP_StatIndicator (Variables|Default|GetUI))) (Utilities|Text|ToText(Float) _returnvalue "HalfToEven"))
    ;[1 1 1] Set Health Progress Bar Percent
    (bind _returnvalue_2 (Class|HealthComponent|GetHealthPercent (Variables|Default|GetCharacterHealth)))
    (Progress|SetPercent (Variables|/Game/UI/GameUI/WBP_StatIndicator.WBP_StatIndicator_C|GethealthProgressBar (Variables|/Game/UI/GameUI/WBP_UserInterface.WBP_UserInterface_C|GetWBP_StatIndicator (Variables|Default|GetUI))) _returnvalue_2)
    (else
      ;[1 1 1] Debug Logging
      (Development|PrintString "BP_PlayerCharacter - Update Health(): UI or CharacterHealth is Invalid"))))

(fn HandlePossession
  (params (Controller :type Controller%20Object%20Reference))
  (bind _ui (Variables|Default|GetUI))
  (bind _ui_2 (Variables|Default|GetUI))
  (bind _asplayer_controller (Utilities|Casting|CastToPlayerController Controller)
    (:then
      (Utilities|IsValid _ui
        (:Is%20Valid
          (Class|UserWidget|SetOwningPlayer _ui _asplayer_controller)
          (if (UserInterface|Viewport|IsinViewport (Variables|Default|GetUI))
            (Development|PrintString "BP_PlayerCharacter - HandlePossession(): UI is already in Viewport")
            (else
              (UserInterface|Viewport|AddtoViewport _ui_2 0)
              (Widget|SetVisibility _ui_2 "Visible"))))
        (:Is%20Not%20Valid
          (Development|PrintString "BP_PlayerCharacter - HandlePossession(): UI Widget is Not Valid"))))
    (:CastFailed
      (Development|PrintString "BP_PlayerCharacter - HandlePossession(): Could not cast to PlayerController"))))

(fn HandleUnpossession
  (params (Old%20Controller :type Controller%20Object%20Reference))
  (Utilities|IsValid (Variables|Default|GetUI)
    (:Is%20Valid
      (Widget|RemovefromParent (Variables|Default|GetUI)))))

(fn ConstructSpells)