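; Player character Blueprint that shows a selected-portrait widget while possessed and visualizes pathfinding with temporary actors.
; The portrait is created on BeginPlay, added to the viewport for the possessing PlayerController and removed on unpossess.
; Health changes copy CharacterHealth's current value and percent into the portrait's text and bar.
; Pathfinding events spawn BP_DeleteLater actors at given transforms, and cleanup destroys every actor of that class in the world.
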(event EventBeginPlay
  (bind _returnvalue (UserInterface|CreateWidget "/Game/UI/GameUI/WBP_SelectedPortrait.WBP_SelectedPortrait_C"))
  (Variables|Default|SetPortraitUI _returnvalue))

(event EventOnPathfinding
  (params (transform :type Transform))
  (Game|SpawnActorfromClass "/Game/Blueprints/BP_DeleteLater.BP_DeleteLater_C" transform "AlwaysSpawn" self 0))

(event EventPossessed
  (params (NewController :type Controller%20Object%20Reference))
  (bind _portraitui (Variables|Default|GetPortraitUI))
  (bind _asplayer_controller (Utilities|Casting|CastToPlayerController NewController)
    (:then
      (Utilities|IsValid (Variables|Default|GetPortraitUI)
        (:Is%20Valid
          (Class|UserWidget|SetOwningPlayer _portraitui _asplayer_controller)
          (UserInterface|Viewport|AddtoViewport _portraitui 0))))
    (:CastFailed
      (Development|PrintString "Event Possessed Cast Failed"))))

(event EventUnpossessed
  (params (OldController :type Controller%20Object%20Reference))
  (bind _portraitui (Variables|Default|GetPortraitUI))
  (Utilities|IsValid _portraitui
    (:Is%20Valid
      (Widget|RemovefromParent _portraitui))))

(event EventCleanupPathfinding
  (bind _outactors (Actor|GetAllActorsOfClass "/Game/Blueprints/BP_DeleteLater.BP_DeleteLater_C"))
  (for _array_element _outactors
    (Actor|DestroyActor _array_element)))

(event EventOnHealthChange
  (Utilities|IsValid (Variables|Default|GetPortraitUI)
    (:Is%20Valid
      (Utilities|IsValid (Variables|Default|GetCharacterHealth)
        (:Is%20Valid
          (bind _returnvalue (Class|HealthComponent|GetCurrentHealth (Variables|Default|GetCharacterHealth)))
          (Rendering|Components|TextRender|SetText (Variables|/Game/UI/GameUI/WBP_SelectedPortrait.WBP_SelectedPortrait_C|GethealthText (Variables|Default|GetPortraitUI)) (Utilities|Text|ToText(Float) _returnvalue "HalfToEven"))
          (bind _returnvalue_2 (Class|HealthComponent|GetHealthPercent (Variables|Default|GetCharacterHealth)))
          (Progress|SetPercent (Variables|/Game/UI/GameUI/WBP_SelectedPortrait.WBP_SelectedPortrait_C|GethealthProgressBar (Variables|Default|GetPortraitUI)) _returnvalue_2))))))

(fn ConstructionScript)